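; A gameplay debugger submenu that shows the ECS targeters owned by the currently selected debug actor.
; It resolves the actor to its entity handle, gathers that entity's targeters and returns one color-coded text line per targeter with its name and targeting status.
; An entity without targeters gets a red placeholder line instead.
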(fn `DoDrawData`
  (params (InParams :type "Ck_GameplayDebugger_DrawSubmenuData_Params Structure (by ref)"))
  (returns (ReturnValue :type "Ck_GameplayDebugger_DrawSubmenuData_Result Structure"))
  (locals (L_CurrentlySelectedDebugActor :type "Actor Object Reference") (L_DebugDataToDraw :type "Array of Text") (L_SelectedActorEntity :type "Ck_Handle Structure") (L_TargeterName :type "GameplayTag Structure") (L_Targeters :type "Array of Ck_Handle_Targeter Structure"))
  (`parent.DoDrawData` InParams)
  (bind _output_get (set `local.L_CurrentlySelectedDebugActor` (`._CurrentlySelectedDebugActor` (break `Ck_GameplayDebugger_DrawSubmenuData_Params` InParams))))
  (`/Engine/EditorBlueprintResources/StandardMacros.IsValid` _output_get
    (:`Is Valid`
      (bind _returnvalue (`/CkFoundation/CkEcs/EntityHandle_CkEcs_ML.TryGet_ActorEntityHandle` (`local.L_CurrentlySelectedDebugActor`))
        (:`Valid`
          (bind _output_get_2 (set `local.L_SelectedActorEntity` _returnvalue))
          (bind _returnvalue_2 (`Ck_Utils_Targeter_UE.ForEach_Targeter` _output_get_2))
          (bind _output_get_3 (set `local.L_Targeters` _returnvalue_2))
          (`/CkFoundation/CkCore/Container/Container_CkCore_ML.Array_IsEmpty_Exec` _output_get_3
            (:`Empty`
              (`KismetArrayLibrary.Array_Add` (`local.L_DebugDataToDraw`) (`|FormatText` "`{red`}<no targeters>")))
            (:`NotEmpty`
              _))
          (for _array_element (`local.L_Targeters`)
            (set `local.L_TargeterName` (`Ck_Utils_GameplayLabel_UE.Get_Label` _array_element))
            (`KismetArrayLibrary.Array_Add` (`local.L_DebugDataToDraw`) (`|FormatText` "`{white`}{name}: {status}" (`BlueprintGameplayTagLibrary.GetTagName` (`local.L_TargeterName`)) (select `ECk_Targeter_TargetingStatus` (`Ck_Utils_Targeter_UE.Get_TargetingStatus` _array_element) :`Targeting` (`|FormatText` "`{green`}TARGETING") :`NotTargeting` (`|FormatText` "`{red`}NOT TARGETING")))))
          (return (make `Ck_GameplayDebugger_DrawSubmenuData_Result` (`local.L_DebugDataToDraw`))))))))