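; Debug action that previews all markers on the currently selected debug actor.
; On perform, it takes the selected index from the debug actor list and proceeds only if that index is valid.
; It then checks the actor is valid and ECS-ready, gets its ECS entity handle, and calls PreviewAllMarkers on it.
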(event `self.DoPerformDebugAction`
  (params (InParams :type "Ck_GameplayDebugger_PerformDebugAction_Params Structure (by ref)"))
  (bind (__debugactorlist __currentlyselecteddebugactorindex) (break `Ck_GameplayDebugger_PerformDebugAction_Params` InParams))
  (`parent.DoPerformDebugAction` InParams)
  (bind _output (`/CkFoundation/CkCore/Container/BPML_CkCore_Container.Array_GetValidatedIndex` (`._DebugActors` (break `Ck_GameplayDebugger_DebugActorList` __debugactorlist)) __currentlyselecteddebugactorindex)
    (:`IsValid`
      (`self.DoPreviewAllMarkersOnSelectedActor` _output))))

(fn `DoPreviewAllMarkersOnSelectedActor`
  (params (InSelectedActor :type "Actor Object Reference"))
  (locals (L_SelectedActorEntity :type "Ck_Handle Structure"))
  (`/Engine/EditorBlueprintResources/StandardMacros.IsValid` InSelectedActor
    (:`Is Valid`
      (if (`Ck_Utils_OwningActor_UE.Get_IsActorEcsReady` InSelectedActor)
        (set `local.L_SelectedActorEntity` (`Ck_Utils_OwningActor_UE.Get_ActorEcsHandle` (`local.InSelectedActor`)))
        (`Ck_Utils_Marker_UE.PreviewAllMarkers` null (`local.L_SelectedActorEntity`))))))