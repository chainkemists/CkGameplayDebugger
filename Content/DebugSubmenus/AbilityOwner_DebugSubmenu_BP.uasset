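; Gameplay debugger submenu for inspecting the ability-owner status of the selected debug actor.
; Each draw resets the level counter and debug text, then resolves the actor's entity handle.
; A valid handle returns the text, adding only a red "not ability owner" line when the ownership check fails.
; A level-to-text helper builds a string per nesting level, but appends empty strings and is never called here.
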(fn `DoDrawData`
  (params (InParams :type "Ck_GameplayDebugger_DrawSubmenuData_Params Structure (by ref)"))
  (returns (ReturnValue :type "Ck_GameplayDebugger_DrawSubmenuData_Result Structure"))
  (locals (L_EntityHandle :type " Structure"))
  (`self.DoResetSharedVariables`)
  (bind _returnvalue (`/CkFoundation/CkEcs/EntityHandle_CkEcs_ML.TryGet_ActorEntityHandle` (`._CurrentlySelectedDebugActor` (break `Ck_GameplayDebugger_DrawSubmenuData_Params` InParams)))
    (:`Valid`
      (if (not (`Ck_Utils_DeferredEntity_UE.Has` _returnvalue))
        (`KismetArrayLibrary.Array_Add` (`self.DebugText`) (`|FormatText` "`{red`}<not ability owner>")))
      (return (make `Ck_GameplayDebugger_DrawSubmenuData_Result` (`self.DebugText`))))))

(fn `DoGet_LevelToText`
  (params (InCurrentlLevel :type Integer))
  (returns (Return :type Text))
  (locals (L_LevelString :type String) (NewLocalVar :type Text))
  (`/CkFoundation/CkCore/Container/Container_CkCore_ML.ForLoop_C++` 0 "LessThan" InCurrentlLevel
    (:`LoopBody`
      (set `local.L_LevelString` (`KismetStringLibrary.Concat_StrStr` (`local.L_LevelString`) "    ")))
    (:`Completed`
      (return (`KismetTextLibrary.Conv_StringToText` (`local.L_LevelString`))))))

(fn `DoResetSharedVariables`
  (set `self.CurrentlLevel` 0)
  (`KismetArrayLibrary.Array_Clear` (`self.DebugText`)))