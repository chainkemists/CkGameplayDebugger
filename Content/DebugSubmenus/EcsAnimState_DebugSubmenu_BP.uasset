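; Gameplay debugger submenu that shows the ECS animation state of the currently selected debug actor.
; DoDrawData resolves the actor's entity handle, then formats its anim Goal, Cluster, State and Overlay gameplay tags into one color-coded line.
; A red "no anim states" message appears when the actor is not ECS-ready or its entity lacks anim-state data.
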(fn `DoDrawData`
  (params (InParams :type "Ck_GameplayDebugger_DrawSubmenuData_Params Structure (by ref)"))
  (returns (ReturnValue :type "Ck_GameplayDebugger_DrawSubmenuData_Result Structure"))
  (locals (L_DebugActor :type "Actor Object Reference") (L_DebugActorEntity :type "Ck_Handle Structure") (L_DataToDraw :type "Array of Text"))
  (bind _l_debugactor (`local.L_DebugActor`))
  (bind _output_get (set `local.L_DebugActor` (`._CurrentlySelectedDebugActor` (break `Ck_GameplayDebugger_DrawSubmenuData_Params` InParams))))
  (`/Engine/EditorBlueprintResources/StandardMacros.IsValid` _output_get
    (:`Is Valid`
      (if (`Ck_Utils_OwningActor_UE.Get_IsActorEcsReady` _l_debugactor)
        (bind _returnvalue (`/CkFoundation/CkEcs/EntityHandle_CkEcs_ML.TryGet_ActorEntityHandle` _l_debugactor)
          (:`Valid`
            (set `local.L_DebugActorEntity` _returnvalue)
            (if (`Ck_Utils_AnimState_UE.Has` (`local.L_DebugActorEntity`))
              (return (make `Ck_GameplayDebugger_DrawSubmenuData_Result` (`|MakeArray` (`|FormatText` "{goal} {cluster} {state} {overlay}" (`|FormatText` "`{grey`}Goal: `{white`}[`{yellow`}{goal}`{white`}]" (`BlueprintGameplayTagLibrary.GetTagName` (`._AnimGoal` (break `Ck_AnimState_Goal` (`Ck_Utils_AnimState_UE.Get_AnimGoal` (`local.L_DebugActorEntity`)))))) (`|FormatText` "`{grey`}Cluster: `{white`}[`{yellow`}{cluster}`{white`}]" (`BlueprintGameplayTagLibrary.GetTagName` (`._AnimCluster` (break `Ck_AnimState_Cluster` (`Ck_Utils_AnimState_UE.Get_AnimCluster` (`local.L_DebugActorEntity`)))))) (`|FormatText` "`{grey`}State: `{white`}[`{yellow`}{state}`{white`}]" (`BlueprintGameplayTagLibrary.GetTagName` (`._AnimState` (break `Ck_AnimState_State` (`Ck_Utils_AnimState_UE.Get_AnimState` (`local.L_DebugActorEntity`)))))) (`|FormatText` "`{grey`}Overlay: `{white`}[`{yellow`}{overlay}`{white`}]" (`BlueprintGameplayTagLibrary.GetTagName` (`._AnimOverlay` (break `Ck_AnimState_Overlay` (`Ck_Utils_AnimState_UE.Get_AnimOverlay` (`local.L_DebugActorEntity`))))))))))
              (else
                _)))))
      (return (make `Ck_GameplayDebugger_DrawSubmenuData_Result` (`|MakeArray` (`|FormatText` "`{red`}<no anim states>")))))))