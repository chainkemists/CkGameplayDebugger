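; Gameplay debugger filter that, going by its name, gathers on-screen actors of a class that are ECS-ready.
; It overrides DoGatherAndFilterActors, takes the parent filter's actor list, and keeps only actors with a valid entity handle.
; The surviving actors are returned as a new debug actor list.
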(fn `DoGatherAndFilterActors`
  (params (InParams :type "Ck_GameplayDebugger_GatherAndFilterActors_Params Structure (by ref)"))
  (returns (ReturnValue :type "Ck_GameplayDebugger_GatherAndFilterActors_Result Structure"))
  (locals (L_FilteredActors :type "Array of Actor Object Reference"))
  (bind _returnvalue (`parent.DoGatherAndFilterActors` InParams))
  (for _array_element (`._DebugActors` (break `Ck_GameplayDebugger_DebugActorList` (`._FilteredDebugActors` (break `Ck_GameplayDebugger_GatherAndFilterActors_Result` _returnvalue))))
    (`/CkFoundation/CkEcs/EntityHandle_CkEcs_ML.TryGet_ActorEntityHandle` _array_element
      (:`Valid`
        (`KismetArrayLibrary.Array_Add` (`local.L_FilteredActors`) _array_element))))
  (return (make `Ck_GameplayDebugger_GatherAndFilterActors_Result` (make `Ck_GameplayDebugger_DebugActorList` (`local.L_FilteredActors`)))))