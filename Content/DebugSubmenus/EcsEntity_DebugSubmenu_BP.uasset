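; Gameplay debugger submenu that shows the ECS entity identity of the currently selected debug actor.
; When the actor is valid and ECS-ready, it reads the actor's ECS handle and draws one color-tagged text line with the entity's ID, number and version.
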(fn `DoDrawData`
  (params (InParams :type "Ck_GameplayDebugger_DrawSubmenuData_Params Structure (by ref)"))
  (returns (ReturnValue :type "Ck_GameplayDebugger_DrawSubmenuData_Result Structure"))
  (locals (L_DebugActor :type "Actor Object Reference"))
  (bind _l_debugactor (`local.L_DebugActor`))
  (bind (_outentityid _outentitynumber _outentityversion) (`Ck_Utils_Entity_UE.Break_Entity` (`Ck_Utils_Handle_UE.Break_Handle` (`Ck_Utils_OwningActor_UE.Get_ActorEcsHandle` _l_debugactor))))
  (bind _output_get (set `local.L_DebugActor` (`._CurrentlySelectedDebugActor` (break `Ck_GameplayDebugger_DrawSubmenuData_Params` InParams))))
  (`/Engine/EditorBlueprintResources/StandardMacros.IsValid` _output_get
    (:`Is Valid`
      (if (`Ck_Utils_OwningActor_UE.Get_IsActorEcsReady` _l_debugactor)
        (return (make `Ck_GameplayDebugger_DrawSubmenuData_Result` (`|MakeArray` (`|FormatText` "`{quartz`}Entity ID: `{green`}{ID} `{LightGrey`}| {Number} ({version})" _outentityid _outentitynumber _outentityversion))))))))