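; A gameplay debugger submenu that shows the ECS transform of the currently selected debug actor.
; DoDrawData resolves the actor's entity handle, validates it and checks it with DoHas before reading the entity's current transform.
; It returns one color-tagged text entry with location, rotation and scale, tinting the X, Y and Z values red, green and blue.
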(fn `DoDrawData`
  (params (InParams :type "Ck_GameplayDebugger_DrawSubmenuData_Params Structure (by ref)"))
  (returns (ReturnValue :type "Ck_GameplayDebugger_DrawSubmenuData_Result Structure"))
  (locals (L_DebugActor :type "Actor Object Reference") (L_DebugActorEntity :type "Ck_Handle Structure") (L_DebugActorTransform :type "Transform Structure") (L_DataToDraw :type "Array of Text"))
  (bind _l_debugactorentity (`local.L_DebugActorEntity`))
  (bind (_x _y _z) (`KismetMathLibrary.BreakVector3f` (.location (`local.L_DebugActorTransform`))))
  (bind (_x_2 _y_2 _z_2) (`KismetMathLibrary.BreakVector3f` (.scale (`local.L_DebugActorTransform`))))
  (bind _output_get (set `local.L_DebugActor` (`._CurrentlySelectedDebugActor` (break `Ck_GameplayDebugger_DrawSubmenuData_Params` InParams))))
  (`/Engine/EditorBlueprintResources/StandardMacros.IsValid` _output_get
    (:`Is Valid`
      (bind _returnvalue (`/CkFoundation/CkEcs/EntityHandle_CkEcs_ML.TryGet_ActorEntityHandle` (`local.L_DebugActor`))
        (:`Valid`
          (bind _output_get_2 (set `local.L_DebugActorEntity` _returnvalue))
          (`/CkFoundation/CkEcs/EntityHandle_CkEcs_ML.ValidateEntityHandle` _output_get_2
            (:`IsValid`
              (if (`Ck_Utils_Transform_UE.DoHas` _l_debugactorentity)
                (set `local.L_DebugActorTransform` (`Ck_Utils_Transform_UE.Get_EntityCurrentTransform` _l_debugactorentity))
                (return (make `Ck_GameplayDebugger_DrawSubmenuData_Result` (`|MakeArray` (`|FormatText` "{loc} {rot} {scale}" (`|FormatText` "`{grey`}Loc: `{white`}[`{red`}{X}`{white`}, `{green`}{Y}`{white`}, `{blue`}{Z}`{white`}]" _x _y _z) (`|FormatText` "`{grey`}Rot: `{white`}[`{red`}{X}`{white`}, `{green`}{Y}`{white`}, `{blue`}{Z}`{white`}]" (.roll (.rotation (`local.L_DebugActorTransform`))) (.pitch (.rotation (`local.L_DebugActorTransform`))) (.yaw (.rotation (`local.L_DebugActorTransform`)))) (`|FormatText` "`{grey`}Scl: `{white`}[`{red`}{X}`{white`}, `{green`}{Y}`{white`}, `{blue`}{Z}`{white`}]" _x_2 _y_2 _z_2)))))))))))))