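; Gameplay debugger submenu that shows the ECS vector attributes of the currently selected debug actor.
; It gets the entity handle from an ECS-ready actor and iterates that entity's vector attributes.
; Each becomes a color-coded line of base, final and bonus values plus the attribute name, with values passed through DoFormatVector.
; An empty list shows a red placeholder that says "float" rather than vector attributes.
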(fn `DoDrawData`
  (params (InParams :type "Ck_GameplayDebugger_DrawSubmenuData_Params Structure (by ref)"))
  (returns (ReturnValue :type "Ck_GameplayDebugger_DrawSubmenuData_Result Structure"))
  (locals (L_CurrentlySelectedDebugActor :type "Actor Object Reference") (L_DebugDataToDraw :type "Array of Text") (L_SelectedActorEntity :type "Ck_Handle Structure") (L_VectorAttributeName :type "GameplayTag Structure") (L_VectorAttributes :type "Array of Ck_Handle Structure"))
  (`parent.DoDrawData` InParams)
  (bind _output_get (set `local.L_CurrentlySelectedDebugActor` (`._CurrentlySelectedDebugActor` (break `Ck_GameplayDebugger_DrawSubmenuData_Params` InParams))))
  (`/Engine/EditorBlueprintResources/StandardMacros.IsValid` _output_get
    (:`Is Valid`
      (if (`Ck_Utils_OwningActor_UE.Get_IsActorEcsReady` (`local.L_CurrentlySelectedDebugActor`))
        (bind _output_get_2 (set `local.L_SelectedActorEntity` (`Ck_Utils_OwningActor_UE.Get_ActorEntityHandleFromSelf` (`local.L_CurrentlySelectedDebugActor`))))
        (if (`Ck_Utils_VectorAttribute_UE.Has_Any` _output_get_2)
          (bind _returnvalue (`Ck_Utils_VectorAttribute_UE.ForEach_VectorAttribute` _output_get_2))
          (bind _output_get_3 (set `local.L_VectorAttributes` _returnvalue))
          (`/CkFoundation/CkCore/Container/Container_CkCore_ML.Array_IsEmpty_Exec` _output_get_3
            (:`Empty`
              (`KismetArrayLibrary.Array_Add` (`local.L_DebugDataToDraw`) (`|FormatText` "`{red`}<no float attributes>")))
            (:`NotEmpty`
              _))
          (for _array_element (`local.L_VectorAttributes`)
            (set `local.L_VectorAttributeName` (`Ck_Utils_GameplayLabel_UE.Get_Label` _array_element))
            (`KismetArrayLibrary.Array_Add` (`local.L_DebugDataToDraw`) (`|FormatText` "`{grey`}{base} `{white`}--> `{yellow`}{final} `{green`}(+{bonus}) `{SpicyPink`}{name}" (`self.DoFormatVector` (`Ck_Utils_VectorAttribute_UE.Get_BaseValue` (`local.L_SelectedActorEntity`) (`local.L_VectorAttributeName`))) (`self.DoFormatVector` (`Ck_Utils_VectorAttribute_UE.Get_FinalValue` (`local.L_SelectedActorEntity`) (`local.L_VectorAttributeName`))) (`self.DoFormatVector` (`Ck_Utils_VectorAttribute_UE.Get_BonusValue` (`local.L_SelectedActorEntity`) (`local.L_VectorAttributeName`))) (`BlueprintGameplayTagLibrary.GetTagName` (`local.L_VectorAttributeName`))))))
        (return (make `Ck_GameplayDebugger_DrawSubmenuData_Result` (`local.L_DebugDataToDraw`)))))))