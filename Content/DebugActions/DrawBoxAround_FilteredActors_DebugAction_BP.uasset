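; Debug action that draws boxes around the filtered list of debug actors, highlighting the currently selected one.
; On perform, it runs the parent action, then loops over the valid actors in the passed-in debug actor list.
; Each box is sized from the actor's full bounds, excluding child actors, times a scale factor, and uses a separate color for the selected index.
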(event `self.DoPerformDebugAction`
  (params (InParams :type "Ck_GameplayDebugger_PerformDebugAction_Params Structure (by ref)"))
  (bind (__debugactorlist __currentlyselecteddebugactorindex) (break `Ck_GameplayDebugger_PerformDebugAction_Params` InParams))
  (`parent.DoPerformDebugAction` InParams)
  (for (_array_element _array_index) (`._DebugActors` (break `Ck_GameplayDebugger_DebugActorList` __debugactorlist))
    (`/Engine/EditorBlueprintResources/StandardMacros.IsValid` _array_element
      (:`Is Valid`
        (bind (_origin _boxextent) (`Actor.GetActorBounds` _array_element false false))
        (`KismetSystemLibrary.DrawDebugBox` _origin (* _boxextent (`self.BoundsScale`)) (select `bool` (== _array_index __currentlyselecteddebugactorindex) :`false` (`self.NotSelectedLineColor`) :`true` (`self.SelectedLineColor`)) (struct) 0.0 (`self.LineThickness`))))))