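; Gameplay debugger submenu that lists the ECS timers on the currently selected debug actor's entity.
; DoDrawData resolves the actor's entity handle, gathers all its timer names, and adds one formatted line per timer, or a red "no timers" line.
; Each line shows an ASCII progress bar colored by paused or running state, elapsed and goal times, and the timer name.
; Count-down timers reverse the bar and flip the order of the two times.
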(fn `DoDrawData`
  (params (InParams :type "Ck_GameplayDebugger_DrawSubmenuData_Params Structure (by ref)"))
  (returns (ReturnValue :type "Ck_GameplayDebugger_DrawSubmenuData_Result Structure"))
  (locals (L_CurrentlySelectedDebugActor :type "Actor Object Reference") (L_SelectedActorEntity :type "Ck_Handle Structure") (L_TimerNames :type "Array of GameplayTag Structure") (L_DebugDataToDraw :type "Array of Text"))
  (`parent.DoDrawData` InParams)
  (bind _output_get (set `local.L_CurrentlySelectedDebugActor` (`._CurrentlySelectedDebugActor` (break `Ck_GameplayDebugger_DrawSubmenuData_Params` InParams))))
  (`/Engine/EditorBlueprintResources/StandardMacros.IsValid` _output_get
    (:`Is Valid`
      (bind _returnvalue (`/CkFoundation/CkEcs/BPML_CkEcs_EntityHandle.TryGet_ActorEntityHandle` (`local.L_CurrentlySelectedDebugActor`))
        (:`Valid`
          (bind _output_get_2 (set `local.L_SelectedActorEntity` _returnvalue))
          (bind _output_get_3 (set `local.L_TimerNames` (`Ck_Utils_Timer_UE.Get_All` _output_get_2)))
          (`/CkFoundation/CkCore/Container/BPML_CkCore_Container.Array_IsEmpty_Exec` _output_get_3
            (:`Empty`
              (`KismetArrayLibrary.Array_Add` (`local.L_DebugDataToDraw`) (`|FormatText` "`{red`}<no timers>")))
            (:`NotEmpty`
              _))
          (for _array_element (`local.L_TimerNames`)
            (`KismetArrayLibrary.Array_Add` (`local.L_DebugDataToDraw`) (`self.Get_PrettifiedTimer` _array_element (`local.L_SelectedActorEntity`))))
          (return (make `Ck_GameplayDebugger_DrawSubmenuData_Result` (`local.L_DebugDataToDraw`))))))))

(fn `Get_PrettifiedTimer`
  (params (InTimerName :type "GameplayTag Structure") (InSelectedActorEntity :type "Ck_Handle Structure") (InPrefix :type Text))
  (returns (Result :type Text))
  (locals (L_TimerName :type "GameplayTag Structure") (L_TimerState :type "ECk_Timer_State Enum") (L_NormalizedTimerElapsed :type "Ck_Time Structure") (L_TimerValue :type "Ck_Chrono Structure") (L_SelectedActorEntity :type "Ck_Handle Structure") (L_CountDirection :type "ECk_Timer_CountDirection Enum" :default "CountUp"))
  (bind (_outgoal _outtimeelapsed) (`Ck_Utils_Chrono_UE.Break_Chrono` (`local.L_TimerValue`)))
  (bind _returnvalue (`KismetTextLibrary.Conv_DoubleToText` (`._Seconds` (break `Ck_Time` _outgoal)) "HalfToEven" false true 1 324 2 2))
  (bind _returnvalue_2 (`KismetTextLibrary.Conv_DoubleToText` (`._Seconds` (break `Ck_Time` _outtimeelapsed)) "HalfToEven" false true 1 324 2 2))
  (set `local.L_TimerName` InTimerName)
  (set `local.L_SelectedActorEntity` InSelectedActorEntity)
  (set `local.L_TimerState` (`Ck_Utils_Timer_UE.Get_CurrentState` (`local.L_SelectedActorEntity`) (`local.L_TimerName`)))
  (bind _output_get (set `local.L_TimerValue` (`Ck_Utils_Timer_UE.Get_CurrentTimerValue` (`local.L_SelectedActorEntity`) (`local.L_TimerName`))))
  (set `local.L_NormalizedTimerElapsed` (`Ck_Utils_Chrono_UE.Get_TimeElapsed` _output_get "ZeroToOne"))
  (set `local.L_CountDirection` (`Ck_Utils_Timer_UE.Get_CountDirection` (`local.L_SelectedActorEntity`) (`local.L_TimerName`)))
  (bind _returnvalue_3 (`Ck_Utils_DebugDraw_UE.Create_ASCII_ProgressBar` (make `Ck_FloatRange_0to1` (`._Seconds` (break `Ck_Time` (`local.L_NormalizedTimerElapsed`)))) (`self.ASCIIProgressBarLength`) (select `ECk_Timer_CountDirection` (`local.L_CountDirection`) :`CountUp` "Forward" :`CountDown` "Reverse" :!type "ECk_ForwardReverse Enum")))
  (return (`|FormatText` "{prefix}`{white`}[{stateColor}{progress}`{white`}] {CurrentAndMax} `{SpicyPink`}{name}" (`local.InPrefix`) (select `ECk_Timer_State` (`local.L_TimerState`) :`Paused` (`|FormatText` "`{grey`}") :`Running` (`|FormatText` "`{yellow`}")) (`KismetTextLibrary.Conv_StringToText` _returnvalue_3) (select `ECk_Timer_CountDirection` (`local.L_CountDirection`) :`CountUp` (`|FormatText` "`{grey`}{current}`{white`}/`{yellow`}{max}" _returnvalue_2 _returnvalue) :`CountDown` (`|FormatText` "`{yellow`}{max}`{white`}/`{grey`}{current}" _returnvalue _returnvalue_2)) (`BlueprintGameplayTagLibrary.GetTagName` (`local.L_TimerName`)))))