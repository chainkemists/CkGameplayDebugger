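; Debug action that marks the currently selected debug actor with a vertical arrow.
; It calls the parent action, then fetches the selected actor from the debug actor list using a validated index.
; The arrow is drawn upward from the actor's location, with configurable length, size and thickness.
; Its color oscillates between two configurable colors using a sine of game time as the lerp alpha.
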(event `self.DoPerformDebugAction`
  (params (InParams :type "Ck_GameplayDebugger_PerformDebugAction_Params Structure (by ref)"))
  (bind (__debugactorlist __currentlyselecteddebugactorindex) (break `Ck_GameplayDebugger_PerformDebugAction_Params` InParams))
  (`parent.DoPerformDebugAction` InParams)
  (bind _output (`/CkFoundation/CkCore/Container/BPML_CkCore_Container.Array_GetValidatedIndex` (`._DebugActors` (break `Ck_GameplayDebugger_DebugActorList` __debugactorlist)) __currentlyselecteddebugactorindex)
    (:`IsValid`
      (`self.DoVisualizeSelectedActor` _output))))

(fn `DoVisualizeSelectedActor`
  (params (InSelectedActor :type "Actor Object Reference"))
  (bind _returnvalue (`Actor.K2_GetActorLocation` (`local.InSelectedActor`)))
  (`/Engine/EditorBlueprintResources/StandardMacros.IsValid` InSelectedActor
    (:`Is Valid`
      (`KismetSystemLibrary.DrawDebugArrow` _returnvalue (+ _returnvalue (`KismetMathLibrary.MakeVector` 0.0 0.0 (`self.VisualizerLength`))) (`self.Visualizer Size`) (`KismetMathLibrary.LinearColorLerp` (`self.ColorA`) (`self.ColorB`) (`KismetMathLibrary.Sin` (* (`GameplayStatics.GetTimeSeconds`) (`self.ColorLerpSpeed`)))) 0.0 (`self.VisualizerThickness`)))))