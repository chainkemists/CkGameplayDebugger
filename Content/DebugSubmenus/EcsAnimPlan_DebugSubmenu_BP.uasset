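; Gameplay debugger submenu that lists the ECS anim plans owned by the currently selected debug actor.
; It resolves the actor's entity handle, iterates its anim plans and draws one color-coded line per plan with its Goal, Cluster and State tags.
; An actor with no anim plans shows a red placeholder line instead.
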(fn `DoDrawData`
  (params (InParams :type "Ck_GameplayDebugger_DrawSubmenuData_Params Structure (by ref)"))
  (returns (ReturnValue :type "Ck_GameplayDebugger_DrawSubmenuData_Result Structure"))
  (locals (L_DebugActor :type "Actor Object Reference") (L_DebugActorEntity :type "Ck_Handle Structure") (L_DataToDraw :type "Array of Text") (L_CurrentlySelectedDebugActor :type "Actor Object Reference") (L_AnimPlans :type "Array of Ck_Handle_AnimPlan Structure"))
  (`parent.DoDrawData` InParams)
  (bind _output_get (set `local.L_CurrentlySelectedDebugActor` (`._CurrentlySelectedDebugActor` (break `Ck_GameplayDebugger_DrawSubmenuData_Params` InParams))))
  (`/Engine/EditorBlueprintResources/StandardMacros.IsValid` _output_get
    (:`Is Valid`
      (bind _returnvalue (`/CkFoundation/CkEcs/EntityHandle_CkEcs_ML.TryGet_ActorEntityHandle` (`local.L_CurrentlySelectedDebugActor`))
        (:`Valid`
          (bind _returnvalue_2 (`Ck_Utils_AnimPlan_UE.ForEach_AnimPlan` _returnvalue))
          (bind _output_get_2 (set `local.L_AnimPlans` _returnvalue_2))
          (`/CkFoundation/CkCore/Container/Container_CkCore_ML.Array_IsEmpty_Exec` _output_get_2
            (:`Empty`
              (`KismetArrayLibrary.Array_Add` (`local.L_DataToDraw`) (`|FormatText` "`{red`}<no anim plans>")))
            (:`NotEmpty`
              _))
          (for _array_element (`local.L_AnimPlans`)
            (`KismetArrayLibrary.Array_Add` (`local.L_DataToDraw`) (`self.Get_PrettifiedAnimPlan` _array_element)))
          (return (make `Ck_GameplayDebugger_DrawSubmenuData_Result` (`local.L_DataToDraw`))))))))

(fn `Get_PrettifiedAnimPlan`
  (params (InAnimPlanEntity :type "Ck_Handle_AnimPlan Structure") (InPrefix :type Text))
  (returns (Result :type Text))
  (locals (L_AnimPlanEntity :type "Ck_Handle_AnimPlan Structure"))
  (bind (_returnvalue__animgoal _returnvalue__animcluster _returnvalue__animstate) (break `Ck_AnimPlan_State` (`Ck_Utils_AnimPlan_UE.Get_AnimState` InAnimPlanEntity)))
  (return (`|FormatText` "{prefix}`{white`}Goal:`{yellow`}{goal} `{white`}Cluster:`{yellow`}{cluster} `{white`}State:`{yellow`}{state} " InPrefix (`BlueprintGameplayTagLibrary.GetTagName` _returnvalue__animgoal) (`BlueprintGameplayTagLibrary.GetTagName` _returnvalue__animcluster) (`BlueprintGameplayTagLibrary.GetTagName` _returnvalue__animstate))))