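; Gameplay debugger submenu that lists the selected debug actor's abilities as colored text.
; DoDrawData resets shared state, then recursively walks the actor entity's abilities, tracking nesting depth for the line prefix.
; Each line shows name, replication, execution and activation policies, green when active.
; An ability's timers print through the ECS timers submenu's class default object; nested abilities are visited only when it has no timers.
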(event `DoPopulateAbilityOwnerData`
  (params (InAbilityOwnerHandle :type "Ck_Handle Structure"))
  (`Ck_Utils_AbilityOwner_UE.ForEach_Ability` InAbilityOwnerHandle (delegate `OnEachAbility`)))

(event `OnEachAbility`
  (params (InAbilityHandle :type "Ck_Handle Structure"))
  (`self.Do Populate Ability` (stale `DoPopulateAbilityOwnerData` InAbilityOwnerHandle) InAbilityHandle))

(fn `Do Populate Ability`
  (params (InAbilityOwner :type "Ck_Handle Structure (by ref)") (InAbility :type "Ck_Handle Structure"))
  (bind _inability (`local.InAbility`))
  (bind _inability_2 (`local.InAbility`))
  (if (`Ck_Utils_Handle_UE.Get_Handle_IsNotEqual` InAbilityOwner InAbility)
    (`KismetArrayLibrary.Array_Add` (`self.DebugText`) (`self.DoGetPrettifiedAbility` (`self.CurrentlLevel`) (`Ck_Utils_GameplayLabel_UE.Get_Label` _inability) (`Ck_Utils_Ability_UE.Get_NetworkSettings` _inability) (`Ck_Utils_Ability_UE.Get_ActivationSettings` _inability) (`Ck_Utils_Ability_UE.Get_Status` _inability)))
    (if (and (`Ck_Utils_Timer_UE.Has_Any` _inability_2) (`KismetArrayLibrary.Array_IsNotEmpty` (`Ck_Utils_Timer_UE.Get_All` _inability_2)))
      (for _array_element (`Ck_Utils_Timer_UE.Get_All` (`local.InAbility`))
        (`KismetArrayLibrary.Array_Add` (`self.DebugText`) (`/CkDebugger/DebugSubmenus/EcsTimers_DebugSubmenu_BP.GetPrettifiedTimer` (`Ck_Utils_Object_UE.DoGet_ClassDefaultObject` "/CkDebugger/DebugSubmenus/EcsTimers_DebugSubmenu_BP.EcsTimers_DebugSubmenu_BP_C") _array_element (`local.InAbility`) (`self.DoGetLevelToText` (`self.CurrentlLevel`)))))
      (elif (`Ck_Utils_AbilityOwner_UE.Has` (`local.InAbility`))
        (`/Engine/EditorBlueprintResources/StandardMacros.IncrementInt` (`self.CurrentlLevel`)
          (:`  `
            (`self.DoPopulateAbilityOwnerData` (`local.InAbility`))
            (`/Engine/EditorBlueprintResources/StandardMacros.DecrementInt` (`self.CurrentlLevel`))))))))

(fn `DoDrawData`
  (params (InParams :type "Ck_GameplayDebugger_DrawSubmenuData_Params Structure (by ref)"))
  (returns (ReturnValue :type "Ck_GameplayDebugger_DrawSubmenuData_Result Structure"))
  (locals (L_EntityHandle :type "Ck_Handle Structure") (L_ActiveAbilities :type "Array of GameplayTag Structure") (L_InactiveAbiilties :type "Array of GameplayTag Structure"))
  (`self.DoResetSharedVariables`)
  (bind _returnvalue (`/CkFoundation/CkEcs/BPML_CkEcs_EntityHandle.TryGet_ActorEntityHandle` (`._CurrentlySelectedDebugActor` (break `Ck_GameplayDebugger_DrawSubmenuData_Params` InParams)))
    (:`Valid`
      (bind _output_get (set `local.L_EntityHandle` _returnvalue))
      (`self.DoPopulateAbilityOwnerData` _output_get)
      (return (make `Ck_GameplayDebugger_DrawSubmenuData_Result` (`self.DebugText`))))))

(fn `DoGetLevelToText`
  (params (InCurrentlLevel :type Integer))
  (returns (Return :type Text))
  (locals (L_LevelString :type String) (NewLocalVar :type Text))
  (`/CkFoundation/CkCore/Container/BPML_CkCore_Container.ForLoop_C++` 0 "LessThan" InCurrentlLevel
    (:`LoopBody`
      (set `local.L_LevelString` (`KismetStringLibrary.Concat_StrStr` (`local.L_LevelString`) "    ")))
    (:`Completed`
      (return (`KismetTextLibrary.Conv_StringToText` (`local.L_LevelString`))))))

(fn `DoGetPrettifiedAbility`
  (params (InCurrentLevel :type Integer) (InGameplayTag :type "GameplayTag Structure (by ref)") (InNetworkSettings :type "Ck_Ability_NetworkSettings Structure (by ref)") (InActivationSettings :type "Ck_Ability_ActivationSettings Structure (by ref)") (InAbilityStatus :type "ECk_Ability_Status Enum" :default "NotActive"))
  (returns (Result :type Text))
  (locals (L_Data :type "Array of Text"))
  (bind (__replicationtype __executionpolicy) (break `Ck_Ability_NetworkSettings` InNetworkSettings))
  (return (`|FormatText` "`{grey`}{Level}{active_color}{AbilityName} `{grey`}[RepType:{ReplicationType}] [ExecPolicy:{ExecutionPolicy}] [{ActivationSettings}]" (`self.DoGetLevelToText` (`local.InCurrentLevel`)) (select `ECk_Ability_Status` (`local.InAbilityStatus`) :`NotActive` "{white}" :`Active` "{green}") (`BlueprintGameplayTagLibrary.GetTagName` InGameplayTag) (`|GetEnumeratorNameAsString` __replicationtype) (`|GetEnumeratorNameAsString` __executionpolicy) (`|GetEnumeratorNameAsString` (`._ActivationPolicy` (break `Ck_Ability_ActivationSettings` InActivationSettings))))))

(fn `DoResetSharedVariables`
  (set `self.CurrentlLevel` 0)
  (`KismetArrayLibrary.Array_Clear` (`self.DebugText`)))