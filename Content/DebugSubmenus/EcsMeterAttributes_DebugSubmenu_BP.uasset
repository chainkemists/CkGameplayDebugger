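; Debug submenu that lists the ECS meter attributes of the actor currently selected in the gameplay debugger.
; For an ECS-ready actor, it gets every meter attribute on its entity and reads each final value.
; Each becomes a color-coded line with an ASCII fill bar, min and max capacity, current value and tag name.
; An entity without meters shows a red placeholder line instead.
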(fn `DoDrawData`
  (params (InParams :type "Ck_GameplayDebugger_DrawSubmenuData_Params Structure (by ref)"))
  (returns (ReturnValue :type "Ck_GameplayDebugger_DrawSubmenuData_Result Structure"))
  (locals (L_CurrentlySelectedDebugActor :type "Actor Object Reference") (L_MeterAttributeNames :type "Array of GameplayTag Structure") (L_DebugDataToDraw :type "Array of Text") (L_SelectedActorEntity :type "Ck_Handle Structure") (L_MeterAttributeName :type "GameplayTag Structure") (L_MeterFinalValue :type "Ck_Meter Structure"))
  (bind (_outmetercapacity _outmetercurrentvalue) (`Ck_Utils_Meter_UE.Break_Meter` (`local.L_MeterFinalValue`)))
  (bind (__mincapacity __maxcapacity) (break `Ck_Meter_Capacity` _outmetercapacity))
  (`parent.DoDrawData` InParams)
  (bind _output_get (set `local.L_CurrentlySelectedDebugActor` (`._CurrentlySelectedDebugActor` (break `Ck_GameplayDebugger_DrawSubmenuData_Params` InParams))))
  (`/Engine/EditorBlueprintResources/StandardMacros.IsValid` _output_get
    (:`Is Valid`
      (if (`Ck_Utils_OwningActor_UE.Get_IsActorEcsReady` (`local.L_CurrentlySelectedDebugActor`))
        (bind _output_get_2 (set `local.L_SelectedActorEntity` (`Ck_Utils_OwningActor_UE.Get_ActorEcsHandle` (`local.L_CurrentlySelectedDebugActor`))))
        (bind _output_get_3 (set `local.L_MeterAttributeNames` (`Ck_Utils_MeterAttribute_UE.Get_All` _output_get_2)))
        (`/CkFoundation/CkCore/Container/BPML_CkCore_Container.Array_IsEmpty_Exec` _output_get_3
          (:`Empty`
            (`KismetArrayLibrary.Array_Add` (`local.L_DebugDataToDraw`) (`|FormatText` "`{red`}<no meter attributes>")))
          (:`NotEmpty`
            _))
        (for _array_element (`local.L_MeterAttributeNames`)
          (set `local.L_MeterAttributeName` _array_element)
          (bind _output_get_4 (set `local.L_MeterFinalValue` (`Ck_Utils_MeterAttribute_UE.Get_FinalValue` (`local.L_MeterAttributeName`) (`local.L_SelectedActorEntity`))))
          (bind _returnvalue (`Ck_Utils_DebugDraw_UE.Create_ASCII_ProgressBar` (`Ck_Utils_Meter_UE.Get_MeterPercentageUsed` _output_get_4) (`self.ASCIIProgressBarLength`)))
          (`KismetArrayLibrary.Array_Add` (`local.L_DebugDataToDraw`) (`|FormatText` "`{white`}[`{yellow`}{progress}`{white`}] [`{grey`}{min}`{white`},`{grey`}{max} `{white`}| `{green`}{current}`{white`}] `{SpicyPink`}{name}" (`BlueprintGameplayTagLibrary.GetTagName` (`local.L_MeterAttributeName`)) _returnvalue __mincapacity __maxcapacity (`._CurrentValue` (break `Ck_Meter_Current` _outmetercurrentvalue)))))
        (return (make `Ck_GameplayDebugger_DrawSubmenuData_Result` (`local.L_DebugDataToDraw`)))))))