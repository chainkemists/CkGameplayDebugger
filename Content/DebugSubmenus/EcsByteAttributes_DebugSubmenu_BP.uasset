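; Gameplay debugger submenu that shows the byte attributes of the currently selected debug actor's ECS entity.
; When the actor is ECS-ready, it gets the entity handle and iterates its byte attributes.
; Each attribute becomes a color-coded line with base, final and bonus values plus its tag name, or a red placeholder when none exist.
; The lines are returned as the submenu's draw data.
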(fn `DoDrawData`
  (params (InParams :type "Ck_GameplayDebugger_DrawSubmenuData_Params Structure (by ref)"))
  (returns (ReturnValue :type "Ck_GameplayDebugger_DrawSubmenuData_Result Structure"))
  (locals (L_CurrentlySelectedDebugActor :type "Actor Object Reference") (L_DebugDataToDraw :type "Array of Text") (L_SelectedActorEntity :type "Ck_Handle Structure") (L_ByteAttributeName :type "GameplayTag Structure") (L_ByteAttributes :type "Array of Ck_Handle Structure"))
  (`parent.DoDrawData` InParams)
  (bind _output_get (set `local.L_CurrentlySelectedDebugActor` (`._CurrentlySelectedDebugActor` (break `Ck_GameplayDebugger_DrawSubmenuData_Params` InParams))))
  (`/Engine/EditorBlueprintResources/StandardMacros.IsValid` _output_get
    (:`Is Valid`
      (if (`Ck_Utils_OwningActor_UE.Get_IsActorEcsReady` (`local.L_CurrentlySelectedDebugActor`))
        (bind _output_get_2 (set `local.L_SelectedActorEntity` (`Ck_Utils_OwningActor_UE.Get_ActorEntityHandleFromSelf` (`local.L_CurrentlySelectedDebugActor`))))
        (if (`Ck_Utils_ByteAttribute_UE.Has_Any` _output_get_2)
          (bind _returnvalue (`Ck_Utils_ByteAttribute_UE.ForEach_ByteAttribute` _output_get_2))
          (bind _output_get_3 (set `local.L_ByteAttributes` _returnvalue))
          (`/CkFoundation/CkCore/Container/Container_CkCore_ML.Array_IsEmpty_Exec` _output_get_3
            (:`Empty`
              (`KismetArrayLibrary.Array_Add` (`local.L_DebugDataToDraw`) (`|FormatText` "`{red`}<no byte attributes>")))
            (:`NotEmpty`
              _))
          (for _array_element (`local.L_ByteAttributes`)
            (set `local.L_ByteAttributeName` (`Ck_Utils_GameplayLabel_UE.Get_Label` _array_element))
            (`KismetArrayLibrary.Array_Add` (`local.L_DebugDataToDraw`) (`|FormatText` "`{grey`}{base} `{white`}--> `{yellow`}{final} `{green`}(+{bonus}) `{SpicyPink`}{name}" (`KismetMathLibrary.Conv_ByteToDouble` (`Ck_Utils_ByteAttribute_UE.Get_BaseValue` (`local.L_SelectedActorEntity`) (`local.L_ByteAttributeName`))) (`KismetMathLibrary.Conv_ByteToDouble` (`Ck_Utils_ByteAttribute_UE.Get_FinalValue` (`local.L_SelectedActorEntity`) (`local.L_ByteAttributeName`))) (`KismetMathLibrary.Conv_ByteToDouble` (`Ck_Utils_ByteAttribute_UE.Get_BonusValue` (`local.L_SelectedActorEntity`) (`local.L_ByteAttributeName`))) (`BlueprintGameplayTagLibrary.GetTagName` (`local.L_ByteAttributeName`))))))
        (return (make `Ck_GameplayDebugger_DrawSubmenuData_Result` (`local.L_DebugDataToDraw`)))))))