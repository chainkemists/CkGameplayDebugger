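; A gameplay debugger submenu that displays the ECS float attributes of the currently selected debug actor.
; DoDrawData checks that the actor is valid and ECS-ready, then gets its entity handle and all float attribute names on it.
; Each attribute becomes a color-tagged line showing name, base value, final value and bonus, with a red notice when none exist.
; The lines are returned as the submenu's draw data result.
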(fn `DoDrawData`
  (params (InParams :type "Ck_GameplayDebugger_DrawSubmenuData_Params Structure (by ref)"))
  (returns (ReturnValue :type "Ck_GameplayDebugger_DrawSubmenuData_Result Structure"))
  (locals (L_CurrentlySelectedDebugActor :type "Actor Object Reference") (L_FloatAttributeNames :type "Array of GameplayTag Structure") (L_DebugDataToDraw :type "Array of Text") (L_SelectedActorEntity :type "Ck_Handle Structure") (L_FloatAttributeName :type "GameplayTag Structure"))
  (`parent.DoDrawData` InParams)
  (bind _output_get (set `local.L_CurrentlySelectedDebugActor` (`._CurrentlySelectedDebugActor` (break `Ck_GameplayDebugger_DrawSubmenuData_Params` InParams))))
  (`/Engine/EditorBlueprintResources/StandardMacros.IsValid` _output_get
    (:`Is Valid`
      (if (`Ck_Utils_OwningActor_UE.Get_IsActorEcsReady` (`local.L_CurrentlySelectedDebugActor`))
        (bind _output_get_2 (set `local.L_SelectedActorEntity` (`Ck_Utils_OwningActor_UE.Get_ActorEcsHandle` (`local.L_CurrentlySelectedDebugActor`))))
        (bind _output_get_3 (set `local.L_FloatAttributeNames` (`Ck_Utils_FloatAttribute_UE.Get_All` _output_get_2)))
        (`/CkFoundation/CkCore/Container/BPML_CkCore_Container.Array_IsEmpty_Exec` _output_get_3
          (:`Empty`
            (`KismetArrayLibrary.Array_Add` (`local.L_DebugDataToDraw`) (`|FormatText` "`{red`}NO FLOAT ATTRIBUTES")))
          (:`NotEmpty`
            _))
        (for _array_element (`local.L_FloatAttributeNames`)
          (set `local.L_FloatAttributeName` _array_element)
          (`KismetArrayLibrary.Array_Add` (`local.L_DebugDataToDraw`) (`|FormatText` "`{SpicyPink`}{name}: `{quartz`}{base} `{grey`}--> `{GoldenRod`}{final} `{LimeGreen`}(+{bonus})" (`BlueprintGameplayTagLibrary.GetTagName` (`local.L_FloatAttributeName`)) (`Ck_Utils_FloatAttribute_UE.Get_BaseValue` (`local.L_FloatAttributeName`) (`local.L_SelectedActorEntity`)) (`Ck_Utils_FloatAttribute_UE.Get_FinalValue` (`local.L_FloatAttributeName`) (`local.L_SelectedActorEntity`)) (`Ck_Utils_FloatAttribute_UE.Get_BonusValue` (`local.L_FloatAttributeName`) (`local.L_SelectedActorEntity`)))))
        (return (make `Ck_GameplayDebugger_DrawSubmenuData_Result` (`local.L_DebugDataToDraw`)))))))