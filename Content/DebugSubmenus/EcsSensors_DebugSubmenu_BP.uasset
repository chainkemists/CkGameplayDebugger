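; Gameplay debugger submenu that lists the ECS sensors on the currently selected debug actor.
; DoDrawData gets the actor's ECS handle once it is ECS-ready, then adds one color-coded text line per sensor, or a red placeholder when there are none.
; Helper functions format each line's marker and non-marker overlap counts, enable state, replication type, shape dimensions and relative transform, alongside the sensor's tag name.
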(fn `DoDrawData`
  (params (InParams :type "Ck_GameplayDebugger_DrawSubmenuData_Params Structure (by ref)"))
  (returns (ReturnValue :type "Ck_GameplayDebugger_DrawSubmenuData_Result Structure"))
  (locals (L_CurrentlySelectedDebugActor :type "Actor Object Reference") (L_SelectedActorEntity :type "Ck_Handle Structure") (L_SensorNames :type "Array of GameplayTag Structure") (L_DebugDataToDraw :type "Array of Text") (L_SensorName :type "GameplayTag Structure"))
  (`parent.DoDrawData` InParams)
  (bind _output_get (set `local.L_CurrentlySelectedDebugActor` (`._CurrentlySelectedDebugActor` (break `Ck_GameplayDebugger_DrawSubmenuData_Params` InParams))))
  (`/Engine/EditorBlueprintResources/StandardMacros.IsValid` _output_get
    (:`Is Valid`
      (if (`Ck_Utils_OwningActor_UE.Get_IsActorEcsReady` (`local.L_CurrentlySelectedDebugActor`))
        (bind _output_get_2 (set `local.L_SelectedActorEntity` (`Ck_Utils_OwningActor_UE.Get_ActorEcsHandle` (`local.L_CurrentlySelectedDebugActor`))))
        (bind _output_get_3 (set `local.L_SensorNames` (`Ck_Utils_Sensor_UE.Get_All` _output_get_2)))
        (`/CkFoundation/CkCore/Container/BPML_CkCore_Container.Array_IsEmpty_Exec` _output_get_3
          (:`Empty`
            (`KismetArrayLibrary.Array_Add` (`local.L_DebugDataToDraw`) (`|FormatText` "`{red`}<no sensors>")))
          (:`NotEmpty`
            _))
        (for _array_element (`local.L_SensorNames`)
          (set `local.L_SensorName` _array_element)
          (`KismetArrayLibrary.Array_Add` (`local.L_DebugDataToDraw`) (`|FormatText` "`{grey`}[{markerOverlaps}`{grey`} | {nonMarkerOverlaps}`{grey`}] [{enable}`{grey`}] [{replication}] [{shapeInfo}`{grey`}] {transform} `{SpicyPink`}{name}" (`self.Get_Sensor_EnableDisable_Text` (`local.L_SelectedActorEntity`) (`local.L_SensorName`)) (`self.Get_Sensor_ReplicationType_Text` (`local.L_SelectedActorEntity`) (`local.L_SensorName`)) (`self.Get_Sensor_ShapeInfo_Text` (`local.L_SelectedActorEntity`) (`local.L_SensorName`)) (`self.Get_Sensor_ShapeTransform_Text` (`local.L_SelectedActorEntity`) (`local.L_SensorName`)) (`BlueprintGameplayTagLibrary.GetTagName` (`local.L_SensorName`)) (`self.Get_Sensor_MarkerOverlaps_Text` (`local.L_SelectedActorEntity`) (`local.L_SensorName`)) (`self.Get_Sensor_NonMarkerOverlaps_Text` (`local.L_SelectedActorEntity`) (`local.L_SensorName`)))))
        (return (make `Ck_GameplayDebugger_DrawSubmenuData_Result` (`local.L_DebugDataToDraw`)))))))